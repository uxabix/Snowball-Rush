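; BP_RunnerGameMode is the runner game mode that builds and recycles the floor as a chain of tiles.
; At BeginPlay it spawns a set number of BP_Floor actors, each placed at the previous tile's attach point.
; ExtendFloor appends a new tile and destroys the oldest once the list exceeds the tile count plus two, keeping the number of live tiles bounded.
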(event `self.ReceiveBeginPlay`
  (for _ (range (`self.Number Of Tiles`))
    (`self.Add Floor`)))

(fn `Add Floor`
  (bind _returnvalue (`|SpawnActorFromClass` "/Game/Runner/Blueprints/BP_Floor.BP_Floor_C" (`self.Floor Attach Point`) "Undefined" "MultiplyWithRoot" null null))
  (bind _returnvalue_2 (`/Game/Runner/Blueprints/BP_Floor.Get Attach Point` _returnvalue))
  (set `self.Floor Attach Point` _returnvalue_2)
  (`KismetArrayLibrary.Array_Add` (`self.Floor Tiles`) _returnvalue))

(fn `Extend Floor`
  (bind _floor_tiles (`self.Floor Tiles`))
  (bind _output (`|GetArrayItem` _floor_tiles))
  (`self.Add Floor`)
  (if (> (`KismetArrayLibrary.Array_Length` (`self.Floor Tiles`)) (+ (`self.Number Of Tiles`) 2))
    (`self.K2_DestroyActor` _output)
    (`KismetArrayLibrary.Array_RemoveItem` _floor_tiles _output)))

(fn `UserConstructionScript`)