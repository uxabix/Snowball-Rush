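; BP_PowerUp_Magnet is a pickup that gives the player ball a timed magnet effect in the runner game.
; On overlap with BP_PlayerBall it plays a coin sound, hides itself and raises the ball's ActiveMagnets counter, then lowers it after a short delay.
; It also destroys any BP_Obstacle_Wall it overlaps.
; The pickup is only hidden, never destroyed, and its collision is left unchanged.
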(event `self.ReceiveActorBeginOverlap`
  (params (OtherActor :type "Actor Object Reference"))
  (`|ExecutionSequence`
    (:`then_0`
      (bind _asbp_obstacle_wall (cast `/Game/Runner/Blueprints/Obstacles/BP_Obstacle_Wall` OtherActor))
      (`self.K2_DestroyActor` _asbp_obstacle_wall))
    (:`then_1`
      (bind _asbp_player_ball (cast `/Game/Runner/Blueprints/BP_PlayerBall` OtherActor))
      (bind _output_get (set `self.As BP Player Ball` _asbp_player_ball))
      (`GameplayStatics.PlaySound2D` "/Game/Runner/Meshes/350874__cabled_mess__coin_c_08.350874__cabled_mess__coin_c_08" 1.0 1.0 0.0 null null)
      (`self.SetActorHiddenInGame` true)
      (`/Engine/EditorBlueprintResources/StandardMacros.IncrementInt` (`/Game/Runner/Blueprints/BP_PlayerBall.Active Magnets` _output_get)
        (:`  `
          (`KismetSystemLibrary.Delay` 5.0)
          (`/Engine/EditorBlueprintResources/StandardMacros.DecrementInt` (`/Game/Runner/Blueprints/BP_PlayerBall.Active Magnets` (`self.As BP Player Ball`))))))))

(fn `UserConstructionScript`)